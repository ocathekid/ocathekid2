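; BP_Platform_ is a player-controlled platform pawn that moves sideways on the Go Left/Right input axis.
; On BeginPlay it has the first player controller possess it.
; The axis value scales movement input along the right vector of the control rotation, with pitch zeroed.
; Each axis event also prints a debug message with the current value, while Tick and the construction script are empty.
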(event `Key|D`
  (params (Key :type "Key Structure")))

(event `self.ReceiveBeginPlay`
  (`Controller.Possess` (`GameplayStatics.GetPlayerController` 0) self))

(event `InputAxis|Go Left/Right`
  (params (AxisValue :type "Float (single-precision)"))
  (bind (_returnvalue_roll _returnvalue_pitch _returnvalue_yaw) (`KismetMathLibrary.BreakRotator` (`self.GetControlRotation`)))
  (`self.AddMovementInput` (`KismetMathLibrary.GetRightVector` (`KismetMathLibrary.MakeRotator` _returnvalue_roll 0.0 _returnvalue_yaw)) AxisValue)
  (`KismetSystemLibrary.PrintString` (`KismetStringLibrary.Concat_StrStr` "Moving " (`KismetStringLibrary.Conv_DoubleToString` AxisValue)) true true (struct :`G` 0.66 :`B` 1.0 :`A` 1.0) (stale `self.ReceiveTick` DeltaSeconds)))

(event `self.ReceiveTick`
  (params (DeltaSeconds :type "Float (single-precision)")))

(fn `UserConstructionScript`)